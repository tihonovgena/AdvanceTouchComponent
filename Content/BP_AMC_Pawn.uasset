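; Pawn that exercises AdvanceTouchSubsystem controls, pushing a mesh around by touch; Escape quits.
; BeginPlay registers its touch controllers, and InputTouch events feed handleTouchInput.
; Swipes, two border buttons and two sticks set ForceVector for DoForce, which applies it as mass-independent force, while taps toggle red and blue materials.
; Tick moves the spring arm to the mesh's location, following it without inheriting rotation from it.
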(event `Key|Escape`
  (params (Key :type "Key Structure"))
  ;[0.151 0.151 0.151] GameQuite
  (:`Pressed`
    (`KismetSystemLibrary.QuitGame` null "Quit")))

(event `self.ReceiveTick`
  (params (DeltaSeconds :type "Float (single-precision)"))
  ;[0.2292 0.2292 0.2292] Movement
  (`SceneComponent.K2_SetWorldLocation` (`self.SpringArm`) (`SceneComponent.K2_GetComponentLocation` (`self.StaticMesh`)) false true))

(event `self.ReceiveBeginPlay`
  ;[1 1 1] SETUP TOUCH CONTROLLER
  (`AdvanceTouchSubsystem.SetupTouchControllers` (subsystem `AdvanceTouchSubsystem`) self))

(event `InputTouch`
  (params (Location :type "Vector Structure") (FingerIndex :type "ETouchIndex Enum"))
  ;[1 1 1] ACCEPT INPUT TOUCH
  (:`Pressed`
    (`AdvanceTouchSubsystem.HandleTouchInput` (subsystem `AdvanceTouchSubsystem`) Location FingerIndex self :!label _label))
  (:`Released`
    (goto _label :!via `Released`))
  (:`Moved`
    (goto _label :!via `Moved`)))

(event `self.Tap.OnTap`
  (params (TouchLocation :type "Vector2D Structure"))
  (bind _staticmesh (`self.StaticMesh`))
  ;[1 1 1] TAP
  (`/Engine/EditorBlueprintResources/StandardMacros.FlipFlop`
    (:`A`
      (`PrimitiveComponent.SetMaterial` _staticmesh 0 "/AdvanceTouchControllers/LevelPrototyping/Materials/MI_Solid_Red.MI_Solid_Red"))
    (:`B`
      (`PrimitiveComponent.SetMaterial` _staticmesh 0 "/Game/LevelPrototyping/Materials/MI_Solid_Blue.MI_Solid_Blue"))))

(event `self.Swipe.OnSwipeUp`
  ;[1 1 1] SWIPES
  (set `self.ForceVector` (1.0 0.0 0.0))
  (`self.DoForce` :!label _label_2))

(event `self.RectButton.OnPressed`
  (params (TouchLocation :type "Vector2D Structure"))
  ;[1 1 1] RECT BORDER BUTTON
  (set `self.ForceVector` (-0.5 0.0 1.0))
  (`self.DoForce`))

(event `self.Swipe.OnSwipeDown`
  ;[1 1 1] SWIPES
  (set `self.ForceVector` (-1.0 0.0 0.0))
  (goto _label_2))

(event `self.Swipe.OnSwipeLeft`
  ;[1 1 1] SWIPES
  (set `self.ForceVector` (0.0 -1.0 0.0))
  (goto _label_2))

(event `self.CircleButton.OnPressed`
  (params (TouchLocation :type "Vector2D Structure"))
  ;[1 1 1] CIRCLE BORDER BUTTON
  (set `self.ForceVector` (0.5 0.0 1.0))
  (`self.DoForce`))

(event `self.Swipe.OnSwipeRight`
  ;[1 1 1] SWIPES
  (set `self.ForceVector` (0.0 1.0 0.0))
  (goto _label_2))

(event `self.StickCircleBorder.OnStick`
  (params (AxisX :type "Float (single-precision)") (AxisY :type "Float (single-precision)"))
  ;[1 1 1] STICKS
  (set `self.ForceVector` (* (`KismetMathLibrary.MakeVector` AxisY AxisX) (`self.StickCoef`)))
  (`self.DoForce` :!label _label_3))

(event `self.StickRectBorder.OnStick`
  (params (AxisX :type "Float (single-precision)") (AxisY :type "Float (single-precision)"))
  ;[1 1 1] STICKS
  (set `self.ForceVector` (* (`KismetMathLibrary.MakeVector` AxisY AxisX) (`self.StickCoef`)))
  (goto _label_3))

(fn `DoForce`
  (`PrimitiveComponent.AddForce` (`self.StaticMesh`) (* (`self.ForceVector`) (`self.Force`)) "None" true))

(fn `UserConstructionScript`)